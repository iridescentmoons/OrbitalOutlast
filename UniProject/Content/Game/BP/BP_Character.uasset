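; Player character driven by thrust, with projectile shooting and health; death reloads or opens a level.
; Forward input applies clamped acceleration to the capsule along the actor's forward vector, while sideways input adds controller yaw and roll and clamps actor roll to bank limits.
; Shooting spawns BP_Projectile at the capsule transform.
; Damage updates the health widget created at BeginPlay alongside a HUD, and zero health triggers Death.
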(event `Death`
  (`GameplayStatics.OpenLevelBySoftObjectPtr` "/Game/Level/Default.Default"))

(event `self.ReceiveAnyDamage`
  (params (Damage :type "Float (single-precision)") (DamageType :type "DamageType Object Reference") (InstigatedBy :type "Controller Object Reference") (DamageCauser :type "Actor Object Reference"))
  (bind _output_get (set `self.CurrentHealth` (`KismetMathLibrary.FClamp` (- (`self.CurrentHealth`) Damage) 0.0 (`self.MaxHealth`))))
  (`/Game/Game/UI/BP_health.UpdateHealth` (`self.HealthRef`) _output_get (`self.MaxHealth`))
  (if (<= _output_get 0.0)
    (`self.Death`)))

(event `self.ReceiveBeginPlay`
  (`|ExecutionSequence`
    (:`then_0`
      (bind _returnvalue (`|CreateWidget` "/Game/Game/UI/BP_health.BP_health_C"))
      (bind _output_get (set `self.healthRef` _returnvalue))
      (`UserWidget.AddToViewport` _output_get 0)
      (set `self.CurrentHealth` (`self.MaxHealth`)))
    (:`then_1`
      (bind _returnvalue_2 (`|CreateWidget` "/Game/Game/UI/HUD.HUD_C"))
      (`UserWidget.AddToViewport` _returnvalue_2 0))))

(event `EnhancedInput|/Game/Game/BP/Input/IA_Shoot`
  (params (ActionValue :type Boolean) (ElapsedSeconds :type "Float (double-precision)") (TriggeredSeconds :type "Float (double-precision)") (InputAction :type "InputAction Object Reference" :default "/Game/Game/BP/Input/IA_Shoot.IA_Shoot"))
  (:`Started`
    (`|SpawnActorFromClass` "/Game/Game/BP/BP_Projectile.BP_Projectile_C" (`SceneComponent.K2_GetComponentToWorld` (`self.CapsuleComponent`)) "Undefined" "MultiplyWithRoot" null null)))

(event `InputAxis|MoveForward`
  (params (AxisValue :type "Float (single-precision)"))
  (`PrimitiveComponent.AddForce` (`self.CapsuleComponent`) (* (`KismetMathLibrary.FClamp` AxisValue -0.5) (`self.ThrustSpeed`) (`self.GetActorForwardVector`)) "None" true))

(event `InputAxis|MoveRight`
  (params (AxisValue :type "Float (single-precision)"))
  (bind (_returnvalue_roll _returnvalue_pitch _returnvalue_yaw) (`KismetMathLibrary.BreakRotator` (`self.K2_GetActorRotation`)))
  (bind _returnvalue (* AxisValue 0.7))
  (`self.AddControllerYawInput` _returnvalue)
  (`self.K2_SetActorRotation` (`KismetMathLibrary.MakeRotator` (`KismetMathLibrary.FClamp` _returnvalue_roll -45.0 45.0) _returnvalue_pitch _returnvalue_yaw) true)
  (`self.AddControllerRollInput` _returnvalue))

(fn `UserConstructionScript`)