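; BP_SpawnController periodically spawns meteors at the level's BP_EntitySpawner actors.
; On BeginPlay it caches the spawners and starts a looping timer that runs SpawnMeteor.
; SpawnMeteor picks a random class from SpawnTypeList and a random spawner, adding slight position jitter and random rotation.
; Tick counts BP_Meteor actors every frame and pauses the timer once more than seven exist, with no resume logic.
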(event `self.ReceiveBeginPlay`
  (bind _outactors (`GameplayStatics.GetAllActorsOfClass` "/Game/Game/BP/BP_EntitySpawner.BP_EntitySpawner_C"))
  (set `self.SpawnList` _outactors)
  (bind _returnvalue (`KismetSystemLibrary.K2_SetTimer` null "SpawnMeteor" 2.0 true 1e-05))
  (set `self.SpawnTimer` _returnvalue))

(event `self.ReceiveTick`
  (params (DeltaSeconds :type "Float (single-precision)"))
  (bind _outactors (`GameplayStatics.GetAllActorsOfClass` "/Game/Game/BP/BP_Meteor.BP_Meteor_C"))
  (if (> (`KismetArrayLibrary.Array_Length` _outactors) 7)
    (`KismetSystemLibrary.K2_PauseTimerHandle` (`self.SpawnTimer`))))

(fn `SpawnMeteor`
  (bind (_returnvalue_roll _returnvalue_pitch _returnvalue_yaw) (`KismetMathLibrary.BreakRotator` (`KismetMathLibrary.RandomRotator` false)))
  (`|SpawnActorFromClass` (`|GetArrayItem` (`self.SpawnTypeList`) (`KismetMathLibrary.RandomIntegerInRange` 0 (- (`KismetArrayLibrary.Array_Length` (`self.SpawnTypeList`)) 1))) (`KismetMathLibrary.MakeTransform` (`KismetMathLibrary.RandomPointInBoundingBox` (`self.K2_GetActorLocation` (`|GetArrayItem` (`self.SpawnList`) (`KismetMathLibrary.RandomIntegerInRange` 0 (- (`KismetArrayLibrary.Array_Length` (`self.SpawnList`)) 1)))) (3.0 3.0 0.01)) (`KismetMathLibrary.MakeRotator` _returnvalue_roll 0.0 _returnvalue_yaw)) "AdjustIfPossibleButDontSpawnIfColliding" "MultiplyWithRoot" null null)
  (return))

(fn `UserConstructionScript`)