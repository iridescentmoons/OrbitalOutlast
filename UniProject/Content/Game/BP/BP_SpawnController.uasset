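; Spawn controller that periodically drops BP_Meteor actors at the BP_EntitySpawner points placed in the level.
; BeginPlay caches the spawners and starts a looping timer that calls SpawnMeteor, which spawns at a random spawner with slight position offset and random rotation.
; The random index range includes the list length, so some calls spawn nothing.
; Tick counts live meteors and pauses the timer above a fixed cap, with no resume.
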(event `self.ReceiveBeginPlay`
  (bind _outactors (`GameplayStatics.GetAllActorsOfClass` "/Game/Game/BP/BP_EntitySpawner.BP_EntitySpawner_C"))
  (set `self.SpawnList` _outactors)
  (bind _returnvalue (`KismetSystemLibrary.K2_SetTimer` null "SpawnMeteor" 2.0 true 1e-05))
  (set `self.SpawnTimer` _returnvalue))

(event `self.ReceiveTick`
  (params (DeltaSeconds :type "Float (single-precision)"))
  (bind _outactors (`GameplayStatics.GetAllActorsOfClass` "/Game/Game/BP/BP_Meteor.BP_Meteor_C"))
  (if (> (`KismetArrayLibrary.Array_Length` _outactors) 7)
    (`KismetSystemLibrary.K2_PauseTimerHandle` (`self.SpawnTimer`))))

(fn `SpawnMeteor`
  (bind (_returnvalue_roll _returnvalue_pitch _returnvalue_yaw) (`KismetMathLibrary.BreakRotator` (`KismetMathLibrary.RandomRotator` false)))
  (bind _returnvalue (`KismetArrayLibrary.Array_Length` (`self.SpawnList`)))
  (set `self.RandomInt` (`KismetMathLibrary.RandomIntegerInRange` 0 _returnvalue))
  (for _index (range _returnvalue)
    (if (== _index (`self.RandomInt`))
      (`|SpawnActorFromClass` "/Game/Game/BP/BP_Meteor.BP_Meteor_C" (`KismetMathLibrary.MakeTransform` (`KismetMathLibrary.RandomPointInBoundingBox` (`self.K2_GetActorLocation` (`|GetArrayItem` (`self.SpawnList`) _index)) (3.0 3.0 0.01)) (`KismetMathLibrary.MakeRotator` _returnvalue_roll 0.0 _returnvalue_yaw)) "AdjustIfPossibleButDontSpawnIfColliding" "MultiplyWithRoot" null null)
      (return)))
  (return))

(fn `UserConstructionScript`)