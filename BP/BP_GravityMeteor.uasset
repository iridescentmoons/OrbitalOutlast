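; BP_GravityMeteor is a meteor actor that drifts toward the player character while they are inside its large gravity collider.
; Overlap events set or clear the target, and Tick offsets the meteor frame-rate independently by GravityStrength, feeding a world-space direction into a local offset.
; A second collider still collects physics-simulating static mesh actors, but the force-based pull for them is disconnected.
; ApplyReflection is an empty stub.
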(event `self.ReceiveTick`
  (params (DeltaSeconds :type "Float (single-precision)"))
  ;[1 1 1] Final attempt, component overlap not consistently firing? (something to do with physics not allowing for collider overlap?)
  (`self.Other Actor`
    (:`then`
      (`self.PullTarget`))
    (:`else`)))

(event `PullTarget`
  ;[1 1 1] Final attempt, component overlap not consistently firing? (something to do with physics not allowing for collider overlap?)
  (`self.K2_AddActorLocalOffset` (* (`KismetMathLibrary.Normal` (- (`self.K2_GetActorLocation` (`self.Other Actor`)) (`self.K2_GetActorLocation`))) (`GameplayStatics.GetWorldDeltaSeconds`) (`self.Gravity Strength`))))

(event `self.GravityPullColliderLarge.OnComponentEndOverlap`
  (params (OverlappedComponent :type "PrimitiveComponent Object Reference") (OtherActor :type "Actor Object Reference") (OtherComp :type "PrimitiveComponent Object Reference") (OtherBodyIndex :type Integer))
  ;[1 1 1] Final attempt, component overlap not consistently firing? (something to do with physics not allowing for collider overlap?)
  (if (== OtherActor (`GameplayStatics.GetPlayerCharacter` 0))
    (set `self.Other Actor` null)))

(event `self.GravityPullColliderLarge.OnComponentBeginOverlap`
  (params (OverlappedComponent :type "PrimitiveComponent Object Reference") (OtherActor :type "Actor Object Reference") (OtherComp :type "PrimitiveComponent Object Reference") (OtherBodyIndex :type Integer) (bFromSweep :type Boolean) (SweepResult :type "HitResult Structure (by ref)"))
  ;[1 1 1] Final attempt, component overlap not consistently firing? (something to do with physics not allowing for collider overlap?)
  (if (== OtherActor (`GameplayStatics.GetPlayerCharacter` 0))
    (set `self.Other Actor` OtherActor)))

(event `self.GravityPullCollider.OnComponentBeginOverlap`
  (params (OverlappedComponent :type "PrimitiveComponent Object Reference") (OtherActor :type "Actor Object Reference") (OtherComp :type "PrimitiveComponent Object Reference") (OtherBodyIndex :type Integer) (bFromSweep :type Boolean) (SweepResult :type "HitResult Structure (by ref)"))
  ;[1 1 1] Attempt 2, waste of time
  (`self.GravityField` OtherActor))

(event `GravityField`
  (params (OverlappingActor :type "Actor Object Reference"))
  ;[1 1 1] Attempt 2, waste of time
  (cast `StaticMeshActor` OverlappingActor)
  (if (`SceneComponent.IsSimulatingPhysics` (`Actor.RootComponent` OverlappingActor) "None")
    (`KismetArrayLibrary.Array_Add` (`self.AffectedActors`) OverlappingActor)))

(fn `Apply Reflection`
  (params (HitMeteor :type "/Game/Game/BP/BP_Meteor Object Reference") (SurfaceNormal :type "Vector Structure")))

(fn `UserConstructionScript`)