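; Player ship character with thrust movement, shooting, health, fuel, a pause menu and a slow-time ability.
; Forward input applies capsule force and drains fuel, though empty fuel does not stop thrust here; sideways input steers yaw and roll.
; Shooting spawns single or double projectiles, repeated by a looping timer while held.
; Damage updates the health widget and opens the end level at zero; Q briefly dilates global time, gated by a cooldown.
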(event `Key|P`
  (params (Key :type "Key Structure"))
  (bind _returnvalue (`GameplayStatics.GetPlayerController` 0))
  (:`Pressed`
    (bind _returnvalue_2 (`|CreateWidget` "/Game/Game/UI/w_pausescreen.w_pausescreen_C"))
    (`UserWidget.AddToViewport` _returnvalue_2 0)
    (set `PlayerController.bShowMouseCursor` true _returnvalue)
    (`WidgetBlueprintLibrary.SetInputMode_UIOnlyEx` _returnvalue null)
    (`GameplayStatics.SetGamePaused` true)))

(event `Drain fuel`
  (params (FuelDrainSpeed :type "Float (double-precision)"))
  (if (`self.ShouldDrain`)
    (bind _output_get (set `self.CurrentFuel` (`KismetMathLibrary.FClamp` (- (`self.CurrentFuel`) (* (`KismetMathLibrary.FClamp` FuelDrainSpeed 0.0 (`self.MaxFuel`)) 0.07)) 0.0 (`self.MaxFuel`))))
    (if (== _output_get 0.0)
      (set `self.ShouldDrain` false))))

(event `Death`
  (`GameplayStatics.OpenLevelBySoftObjectPtr` "/Game/Game/UI/EndLevel.EndLevel"))

(event `self.ReceiveAnyDamage`
  (params (Damage :type "Float (single-precision)") (DamageType :type "DamageType Object Reference") (InstigatedBy :type "Controller Object Reference") (DamageCauser :type "Actor Object Reference"))
  (bind _output_get (set `self.CurrentHealth` (`KismetMathLibrary.FClamp` (- (`self.CurrentHealth`) Damage) 0.0 (`self.MaxHealth`))))
  (`/Game/Game/UI/BP_health.UpdateHealth` (`self.HealthRef`) _output_get (`self.MaxHealth`))
  (if (<= _output_get 0.0)
    (`self.Death`)))

(event `self.ReceiveBeginPlay`
  (bind _returnvalue (`|CreateWidget` "/Game/Game/UI/BP_health.BP_health_C"))
  (bind _output_get (set `self.healthRef` _returnvalue))
  (`UserWidget.AddToViewport` _output_get 0)
  (set `self.CurrentHealth` (`self.MaxHealth`))
  (bind _returnvalue_2 (`|CreateWidget` "/Game/Game/UI/BP_FuelBar.BP_FuelBar_C"))
  (bind _output_get_2 (set `self.FuelRef` _returnvalue_2))
  (`UserWidget.AddToViewport` _output_get_2 0))

(event `Key|Q`
  (params (Key :type "Key Structure"))
  ;[1 1 1] Slow time ability, 10 second cooldown (needs a visual timer on screen for cd) - luke
  (:`Pressed`
    (if (`self.TimeSlowCooldown`)
      (`|ExecutionSequence`
        (:`then_0`
          (set `self.TimeSlowCooldown` false)
          (`GameplayStatics.SetGlobalTimeDilation` 0.2)
          (`KismetSystemLibrary.Delay` 1.0)
          (`GameplayStatics.SetGlobalTimeDilation` 1.0))
        (:`then_1`
          (`KismetSystemLibrary.Delay` 10.0)
          (set `self.TimeSlowCooldown` true))))))

(event `EnhancedInput|/Game/Game/BP/Input/IA_Shoot`
  (params (ActionValue :type Boolean) (ElapsedSeconds :type "Float (double-precision)") (TriggeredSeconds :type "Float (double-precision)") (InputAction :type "InputAction Object Reference" :default "/Game/Game/BP/Input/IA_Shoot.IA_Shoot"))
  ;[1 1 1] Firing Logic with full auto and semi auto has some slight issues
  (:`Triggered`
    (if (not (`KismetSystemLibrary.K2_IsValidTimerHandle` (`self.FiringTimer`)))
      (bind _returnvalue (`KismetSystemLibrary.K2_SetTimer` null "SpawnBullet" (`self.FireRate`) true 1e-05))
      (set `self.FiringTimer` _returnvalue)))
  (:`Started`
    (`self.SpawnBullet`))
  (:`Completed`
    (`KismetSystemLibrary.K2_ClearAndInvalidateTimerHandle` (`self.FiringTimer`))))

(event `InputAxis|MoveForward`
  (params (AxisValue :type "Float (single-precision)"))
  ;[1 1 1] Forward Movement bacwards clamped to slow player
  (`self.Drain fuel` AxisValue)
  (`PrimitiveComponent.AddForce` (`self.CapsuleComponent`) (* (`KismetMathLibrary.FClamp` AxisValue -0.5) (`self.ThrustSpeed`) (`self.GetActorForwardVector`)) "None" true))

(event `InputAxis|MoveRight`
  (params (AxisValue :type "Float (single-precision)"))
  (bind (_returnvalue_roll _returnvalue_pitch _returnvalue_yaw) (`KismetMathLibrary.BreakRotator` (`self.K2_GetActorRotation`)))
  (bind _returnvalue (* AxisValue 0.7))
  ;[1 1 1] Ship Rotation for firing has some logic for a roll effect not yet used as its hard to tell if it adds anything to the experience
  (`self.AddControllerYawInput` _returnvalue)
  (`self.K2_SetActorRotation` (`KismetMathLibrary.MakeRotator` (`KismetMathLibrary.FClamp` (+ _returnvalue_roll 1.0) -45.0 45.0) _returnvalue_pitch _returnvalue_yaw) true)
  (`self.AddControllerRollInput` _returnvalue))

(fn `SpawnBullet`
  (if (`self.IsDoubleShot`)
    (`|SpawnActorFromClass` "/Game/Game/BP/BP_Projectile.BP_Projectile_C" (`SceneComponent.K2_GetComponentToWorld` (`self.DoubleShotPoint1`)) "Undefined" "MultiplyWithRoot" null null)
    (`|SpawnActorFromClass` "/Game/Game/BP/BP_Projectile.BP_Projectile_C" (`SceneComponent.K2_GetComponentToWorld` (`self.DoubleShotPoint2`)) "Undefined" "MultiplyWithRoot" null null)
    (else
      (`|SpawnActorFromClass` "/Game/Game/BP/BP_Projectile.BP_Projectile_C" (`SceneComponent.K2_GetComponentToWorld` (`self.CapsuleComponent`)) "Undefined" "MultiplyWithRoot" null null))))

(fn `UserConstructionScript`)