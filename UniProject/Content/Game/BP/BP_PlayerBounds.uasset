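; Play-area boundary that acts as a portal, wrapping the player character, meteors and projectiles to a LinkedPortal.
; An overlap box records each actor's entry location, and Tick tests a line-plane intersection and front-to-back change to detect crossings.
; Teleports remap location and mirror rotation into the linked portal's space, plus control rotation and velocity for the player.
; A Stopper component's hit event applies a forward impulse to physics-simulating game parts.
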(event `self.ReceiveBeginPlay`)

(event `self.ReceiveTick`
  (params (DeltaSeconds :type "Float (single-precision)"))
  (`self.ShouldTeleport`))

(event `self.Co_PlayerBoundary.OnComponentBeginOverlap`
  (params (OverlappedComponent :type "PrimitiveComponent Object Reference") (OtherActor :type "Actor Object Reference") (OtherComp :type "PrimitiveComponent Object Reference") (OtherBodyIndex :type Integer) (bFromSweep :type Boolean) (SweepResult :type "HitResult Structure (by ref)"))
  (bind (_castedactor _checksuccess) (`self.IsGamePart` OtherActor))
  (if _checksuccess
    (`BlueprintMapLibrary.Map_Add` (`self.CollidedActors`) _castedactor (`self.K2_GetActorLocation` _castedactor))))

(event `self.Co_PlayerBoundary.OnComponentEndOverlap`
  (params (OverlappedComponent :type "PrimitiveComponent Object Reference") (OtherActor :type "Actor Object Reference") (OtherComp :type "PrimitiveComponent Object Reference") (OtherBodyIndex :type Integer))
  (set `self.ExitingActor` OtherActor)
  (if (`BlueprintMapLibrary.Map_Contains` (`self.CollidedActors`) OtherActor)
    (`BlueprintMapLibrary.Map_Remove` (`self.CollidedActors`) (`self.ExitingActor`))))

(event `self.Stopper.OnComponentHit`
  (params (HitComponent :type "PrimitiveComponent Object Reference") (OtherActor :type "Actor Object Reference") (OtherComp :type "PrimitiveComponent Object Reference") (NormalImpulse :type "Vector Structure") (Hit :type "HitResult Structure (by ref)"))
  (bind (_castedactor _checksuccess _physicscomp) (`self.IsGamePart` null))
  (if _checksuccess
    (if (`SceneComponent.IsSimulatingPhysics` _physicscomp "None")
      (`PrimitiveComponent.AddImpulse` _physicscomp (* (`self.GetActorForwardVector`) 4500.0) "None" true))))

(fn `IsCrossingPortal`
  (params (CrossingPoint :type "Vector Structure") (WraparoundLocation :type "Vector Structure") (WraparoundNormal :type "Vector Structure") (CurrentActor :type "Actor Object Reference"))
  (returns (CrossingPortal :type Boolean))
  (locals (IsInFront :type Boolean) (WrapAroundPlane :type "Plane Structure") (IsIntersecting :type Boolean) (IsCrossing :type Boolean))
  (set `local.IsInFront` (>= (`KismetMathLibrary.Dot_VectorVector` (- CrossingPoint WraparoundLocation) WraparoundNormal) 0.0))
  (bind _output_get (set `local.WrapAroundPlane` (`KismetMathLibrary.MakePlaneFromPointAndNormal` (`local.WraparoundLocation`) (`local.WraparoundNormal`))))
  (bind _output_get_2 (set `local.IsIntersecting` (`.ReturnValue` (`KismetMathLibrary.LinePlaneIntersection` (`BlueprintMapLibrary.Map_Find` (`self.PastCollided`) CurrentActor) (`local.CrossingPoint`) _output_get))))
  (set `local.IsCrossing` (and _output_get_2 (not (`local.IsInFront`)) (`self.LastInFront`)))
  (set `self.LastInFront` (`local.IsInFront`))
  (`BlueprintMapLibrary.Map_Add` (`self.PastCollided`) (`local.CurrentActor`) (`BlueprintMapLibrary.Map_Find` (`self.CollidedActors`) (`local.CurrentActor`)))
  (return (`local.IsCrossing`)))

(fn `IsGamePart`
  (params (OverlappedActor :type "Actor Object Reference"))
  (returns (CastedActor :type "Actor Object Reference") (CheckSuccess :type Boolean) (PhysicsComp :type "PrimitiveComponent Object Reference"))
  (bind _asbp_character (cast `/Game/Game/BP/BP_Character` OverlappedActor)
    (:`then`
      (set `self.IsPlayer` true)
      (return _asbp_character true (`Character.CapsuleComponent` _asbp_character)))
    (:`CastFailed`
      (bind _asbp_meteor (cast `/Game/Game/BP/BP_Meteor` (`local.OverlappedActor`))
        (:`then`
          (return _asbp_meteor true (`/Game/Game/BP/BP_Meteor.SM_Meteor` _asbp_meteor)))
        (:`CastFailed`
          (bind _asbp_projectile (cast `/Game/Game/BP/BP_Projectile` (`local.OverlappedActor`))
            (:`then`
              (return _asbp_projectile true null))
            (:`CastFailed`
              (return null false null))))))))

(fn `MirrorAxis`
  (params (OldAxes :type "Rotator Structure") (CollisionPoint :type "Vector Structure"))
  (returns (NewAxes :type "Rotator Structure"))
  (locals (RotatorArray :type "Array of Vector Structure"))
  (bind (_x _y _z) (`KismetMathLibrary.BreakRotIntoAxes` OldAxes))
  (bind _rotatorarray (`local.RotatorArray`))
  (bind _output_get (set `local.RotatorArray` (`|MakeArray` _x _y _z)))
  (for _index (range (`KismetArrayLibrary.Array_Length` _output_get))
    (`KismetArrayLibrary.Array_Set` (`local.RotatorArray`) _index (`self.SwitchDirection` (`|GetArrayItem` (`local.RotatorArray`) _index) (`local.CollisionPoint`))))
  (return (`KismetMathLibrary.MakeRotationFromAxes` (`|GetArrayItem` _rotatorarray) (`|GetArrayItem` _rotatorarray 1) (`|GetArrayItem` _rotatorarray 2))))

(fn `ShouldTeleport`
  (locals (CurrentActor :type "Actor Object Reference"))
  (bind _currentactor (`local.CurrentActor`))
  (if (`BlueprintMapLibrary.Map_IsNotEmpty` (`self.CollidedActors`))
    (bind _keys (`BlueprintMapLibrary.Map_Keys` (`self.CollidedActors`)))
    (for _array_element _keys
      (set `local.CurrentActor` _array_element)
      (if (not (`BlueprintMapLibrary.Map_Contains` (`self.PastCollided`) (`local.CurrentActor`)))
        (`BlueprintMapLibrary.Map_Add` (`self.PastCollided`) (`local.CurrentActor`)))
      (bind _crossingportal (`self.IsCrossingPortal` (`self.K2_GetActorLocation` _currentactor) (`BlueprintMapLibrary.Map_Find` (`self.CollidedActors`) _currentactor) (`SceneComponent.GetForwardVector` (`self.ForwardDirection`)) _currentactor))
      (if _crossingportal
        (`self.TeleportActor` (`local.CurrentActor`))))))

(fn `SwitchDirection`
  (params (InitialDirection :type "Vector Structure") (CollisionPoint :type "Vector Structure"))
  (returns (FormattedDirection :type "Vector Structure"))
  (return (`KismetMathLibrary.TransformDirection` (`self.GetTransform` (`self.LinkedPortal`)) (`KismetMathLibrary.MirrorVectorByNormal` (`KismetMathLibrary.MirrorVectorByNormal` (`KismetMathLibrary.InverseTransformDirection` (`self.GetTransform`) InitialDirection) (1.0 0.0 0.0)) (0.0 1.0 0.0)))))

(fn `TeleportActor`
  (params (CurrentActor :type "Actor Object Reference"))
  (bind _returnvalue (`GameplayStatics.GetPlayerController` 0))
  (bind _value (`BlueprintMapLibrary.Map_Find` (`self.CollidedActors`) (`local.CurrentActor`)))
  (bind _asbp_character (cast `/Game/Game/BP/BP_Character` (`GameplayStatics.GetPlayerCharacter` 0) :!pure true))
  (bind _returnvalue_2 (`Pawn.GetMovementComponent` _asbp_character))
  (`self.K2_SetActorTransform` CurrentActor (`KismetMathLibrary.MakeTransform` (`self.UpdateLocation` (`self.K2_GetActorLocation`) _value (`local.CurrentActor`)) (`self.MirrorAxis` (`self.K2_GetActorRotation`) _value) (`self.GetActorScale3D` (`local.CurrentActor`))) false true)
  (if (`self.IsPlayer`)
    (`Controller.SetControlRotation` _returnvalue (`self.MirrorAxis` (`Controller.GetControlRotation` _returnvalue) (`BlueprintMapLibrary.Map_Find` (`self.CollidedActors`) (`local.CurrentActor`))))
    (set `MovementComponent.Velocity` (`self.Update Velocity` (`MovementComponent.Velocity` _returnvalue_2) (`BlueprintMapLibrary.Map_Find` (`self.CollidedActors`) (`local.CurrentActor`)) _asbp_character) _returnvalue_2)))

(fn `Update Velocity`
  (params (OldVelocity :type "Vector Structure") (CollisionPoint :type "Vector Structure") (AppliedActor :type "/Game/Game/BP/BP_Character Object Reference"))
  (returns (NewVelocity :type "Vector Structure"))
  (return (* (`self.SwitchDirection` (`KismetMathLibrary.Normal` OldVelocity) CollisionPoint) (`KismetMathLibrary.VSize` (`self.GetVelocity` AppliedActor)))))

(fn `UpdateLocation`
  (params (OldLocation :type "Vector Structure") (CollisionPoint :type "Vector Structure") (Actor :type "Actor Object Reference"))
  (returns (NewLocation :type "Vector Structure"))
  (bind _returnvalue (`self.GetTransform` Actor))
  (return (+ (* (`KismetMathLibrary.GetDirectionUnitVector` (`local.OldLocation`) (`local.CollisionPoint`)) (`KismetMathLibrary.Vector_Distance` (`local.OldLocation`) (`local.CollisionPoint`))) (`KismetMathLibrary.TransformLocation` (`self.GetTransform` (`self.LinkedPortal`)) (`KismetMathLibrary.InverseTransformLocation` (`KismetMathLibrary.MakeTransform` (`local.Collisionpoint`) (.rotation _returnvalue) (`KismetMathLibrary.MakeVector` (* (.x (.scale _returnvalue)) -1.0) (* (.y (.scale _returnvalue)) -1.0) (.z (.scale _returnvalue)))) CollisionPoint)))))

(fn `UserConstructionScript`)