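; BP_ClusterMeteor is a physics-driven meteor that damages a character on contact and splits into three regular meteors.
; Tick accelerates its mesh along a stored direction, initially the actor's forward vector.
; Overlapping a BP_Meteor applies an impulse and resets that direction, both using the forward vector reflected off the impact normal.
; Hitting a BP_Character deals damage, clears itself from BP_PlayerBounds' PastCollided, then destroys itself and spawns the trio along X.
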(event `self.ReceiveBeginPlay`
  (set `self.CurrentDirection` (`self.GetActorForwardVector`)))

(event `self.ReceiveTick`
  (params (DeltaSeconds :type "Float (single-precision)"))
  (`PrimitiveComponent.AddForce` (`self.SM_Meteor`) (* (`self.CurrentDirection`) 5000.0 DeltaSeconds) "None" true))

(event `self.Collider.OnComponentBeginOverlap`
  (params (OverlappedComponent :type "PrimitiveComponent Object Reference") (OtherActor :type "Actor Object Reference") (OtherComp :type "PrimitiveComponent Object Reference") (OtherBodyIndex :type Integer) (bFromSweep :type Boolean) (SweepResult :type "HitResult Structure (by ref)"))
  (bind (_returnvalue_x _returnvalue_y _returnvalue_z) (`KismetMathLibrary.BreakVector` (`self.K2_GetActorLocation`)))
  (bind (_returnvalue_x_2 _returnvalue_y_2 _returnvalue_z_2) (`KismetMathLibrary.BreakVector` (`self.K2_GetActorLocation`)))
  (bind (_returnvalue_x_3 _returnvalue_y_3 _returnvalue_z_3) (`KismetMathLibrary.BreakVector` (`self.K2_GetActorLocation`)))
  (bind _asbp_meteor (cast `/Game/Game/BP/BP_Meteor` OtherActor)
    (:`then`
      (`self.ApplyReflection` _asbp_meteor SweepResult_ImpactNormal))
    (:`CastFailed`
      (bind _asbp_character (cast `/Game/Game/BP/BP_Character` OtherActor))
      (`GameplayStatics.ApplyDamage` _asbp_character 10.0 null self)
      (bind _outactors (`GameplayStatics.GetAllActorsOfClass` "/Game/Game/BP/BP_PlayerBounds.BP_PlayerBounds_C"))
      (for _array_element _outactors
        (if (`BlueprintMapLibrary.Map_Contains` (`/Game/Game/BP/BP_PlayerBounds.PastCollided` _array_element) self)
          (`BlueprintMapLibrary.Map_Remove` (`/Game/Game/BP/BP_PlayerBounds.PastCollided` _array_element) self)))
      (`self.K2_DestroyActor`)
      (`|SpawnActorFromClass` "/Game/Game/BP/BP_Meteor.BP_Meteor_C" (`KismetMathLibrary.MakeTransform` (`KismetMathLibrary.MakeVector` (+ _returnvalue_x_2 70.0) _returnvalue_y_2 _returnvalue_z_2)) "AdjustIfPossibleButDontSpawnIfColliding" "MultiplyWithRoot" null null)
      (`|SpawnActorFromClass` "/Game/Game/BP/BP_Meteor.BP_Meteor_C" (`KismetMathLibrary.MakeTransform` (`KismetMathLibrary.MakeVector` (+ _returnvalue_x_3 -70.0) _returnvalue_y_3 _returnvalue_z_3)) "AdjustIfPossibleButDontSpawnIfColliding" "MultiplyWithRoot" null null)
      (`|SpawnActorFromClass` "/Game/Game/BP/BP_Meteor.BP_Meteor_C" (`KismetMathLibrary.MakeTransform` (`KismetMathLibrary.MakeVector` (+ _returnvalue_x 0.0) _returnvalue_y _returnvalue_z)) "AdjustIfPossibleButDontSpawnIfColliding" "MultiplyWithRoot" null null))))

(fn `ApplyReflection`
  (params (HitMeteor :type "/Game/Game/BP/BP_Meteor Object Reference") (SurfaceNormal :type "Vector Structure"))
  (bind _returnvalue (`KismetMathLibrary.GetReflectionVector` (`self.GetActorForwardVector`) SurfaceNormal))
  (if (!= HitMeteor self)
    (`PrimitiveComponent.AddImpulse` (`self.SM_Meteor`) (* _returnvalue 1000.0) "None" false)
    (set `self.CurrentDirection` _returnvalue)))

(fn `UserConstructionScript`)